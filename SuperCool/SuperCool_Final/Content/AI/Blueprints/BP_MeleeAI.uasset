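; Melee enemy AI character that attaches a sword to its mesh socket and deals damage through a Capsule overlap.
; MeleeAttack plays one of three montages from an index re-rolled every Tick.
; Any damage plays a random hit montage and counts toward death, regardless of damage amount.
; Death disables collision, plays a montage, swaps the mesh for a shattering destructible, increments BP_Playing's AI counter, then destroys the actor.
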(event `self.ReceiveBeginPlay`
  (`SceneComponent.K2_AttachToComponent` (`self.Sword`) (`self.Mesh`) "swordpoint" "KeepRelative" "KeepRelative" "KeepRelative" true)
  (`SceneComponent.K2_SetRelativeLocationAndRotation` :`self` (`self.Sword`) :`NewLocation` (-10.0 0.0 -5.0)))

(event `self.ReceiveTick`
  (params (DeltaSeconds :type "Float (single-precision)"))
  (set `self.RandomAttackPose` (`KismetMathLibrary.RandomIntegerInRange` 1 3)))

(event `MeleeAttack`
  (bind _randomattackpose (`self.RandomAttackPose`))
  (bind _mesh (`self.Mesh`))
  ;[1 1 1] attack 애니메이션 랜덤으로 발생
  (`|ExecutionSequence`
    (:`then_0`
      (if (== _randomattackpose 1)
        (`|PlayMontage` _mesh "/Game/AI/MeleeAnim/ANIMMontage_MeleeAttack1.ANIMMontage_MeleeAttack1")))
    (:`then_1`
      (if (== _randomattackpose 2)
        (`|PlayMontage` _mesh "/Game/AI/MeleeAnim/ANIMMontage_MeleeAttack2.ANIMMontage_MeleeAttack2")))
    (:`then_2`
      (if (== _randomattackpose 3)
        (`|PlayMontage` _mesh "/Game/AI/MeleeAnim/ANIMMontage_MeleeAttack3.ANIMMontage_MeleeAttack3")))))

(event `AiHitAnim`
  (bind _randomhitpose (`self.RandomHitPose`))
  (bind _mesh (`self.Mesh`))
  (if (not (`self.AiDie`))
    (set `self.RandomHitPose` (`KismetMathLibrary.RandomIntegerInRange` 1 2))
    (`|ExecutionSequence`
      (:`then_0`
        (if (== _randomhitpose 1)
          (`|PlayMontage` _mesh "/Game/AI/MeleeAnim/ANIMMontage_HitMeleeAI1.ANIMMontage_HitMeleeAI1")))
      (:`then_1`
        (if (== _randomhitpose 2)
          (`|PlayMontage` _mesh "/Game/AI/MeleeAnim/ANIMMontage_HitMeleeAI2.ANIMMontage_HitMeleeAI2"))))))

(event `self.ReceiveAnyDamage`
  (params (Damage :type "Float (single-precision)") (DamageType :type "DamageType Object Reference") (InstigatedBy :type "Controller Object Reference") (DamageCauser :type "Actor Object Reference"))
  (`self.AiDieCheck`))

(event `self.Capsule.OnComponentBeginOverlap`
  (params (OverlappedComponent :type "PrimitiveComponent Object Reference") (OtherActor :type "Actor Object Reference") (OtherComp :type "PrimitiveComponent Object Reference") (OtherBodyIndex :type Integer) (bFromSweep :type Boolean) (SweepResult :type "HitResult Structure (by ref)"))
  (`GameplayStatics.ApplyDamage` OtherActor 1.0))

(event `AiDieCheck`
  (bind _capsulecomponent (`self.CapsuleComponent`))
  (bind _mesh (`self.Mesh`))
  (`self.AiHitAnim`)
  (bind _result (`/Engine/EditorBlueprintResources/StandardMacros.IncrementInt` (`self.DamgeCnt`))
    (:`  `
      (bind _output_get (set `self.DamgeCnt` _result))
      (if (== _output_get (`self.AiDieCnt`))
        (`|ExecutionSequence`
          (:`then_0`
            (`PrimitiveComponent.SetCollisionEnabled` _capsulecomponent "NoCollision")
            (`PrimitiveComponent.SetSimulatePhysics` _capsulecomponent false)
            (set `self.Can Attack` false)
            (set `self.CanMove` false))
          (:`then_1`
            (`|PlayMontage` (`self.Mesh`) "/Game/AI/MeleeAnim/ANIMMontageMeleeDie2.ANIMMontageMeleeDie2"
              (:`then`
                (set `self.AiDie` true))
              (:`OnCompleted`
                (message `/Game/AI/Blueprints/IF_ClearFocus.ClearFocusPlayer` (`AIBlueprintHelperLibrary.GetAIController` null))
                (`PrimitiveComponent.SetMaterial` (`self.Mesh`) 0 "/Game/IceCool/Demo/ExampleMaterials/Characters/MI_IceCharacterOpaque.MI_IceCharacterOpaque")
                (`PrimitiveComponent.SetMaterial` (`self.Sword`) 0 "/Game/IceCool/Demo/ExampleMaterials/Characters/MI_IceCharacterOpaque.MI_IceCharacterOpaque")
                (`SceneComponent.SetVisibility` _mesh false false)
                (bind _returnvalue (`AddComponent|NODE_AddDestructibleComponent-0` :`RelativeTransform` (`SceneComponent.GetRelativeTransform` _mesh)))
                (`DestructibleComponent.SetDestructibleMesh` _returnvalue "/Game/AI/Mesh/MeleeStatic_DM.MeleeStatic_DM")
                (`PrimitiveComponent.SetSimulatePhysics` _returnvalue true)
                (`DestructibleComponent.ApplyDamage` _returnvalue 60.0 (`SceneComponent.K2_GetComponentLocation` (`self.Mesh`)) (`KismetMathLibrary.MakeVector` (`KismetMathLibrary.SelectFloat` 0.0 1.0 (`KismetMathLibrary.RandomBool`)) (`KismetMathLibrary.SelectFloat` 0.0 1.0 (`KismetMathLibrary.RandomBool`)) (`KismetMathLibrary.SelectFloat` 0.0 1.0 (`KismetMathLibrary.RandomBool`))) 600.0)
                (bind _returnvalue_2 (`GameplayStatics.GetActorOfClass` "/Game/Blueprints/BP_Playing.BP_Playing_C"))
                (bind _result_2 (`/Engine/EditorBlueprintResources/StandardMacros.IncrementInt` (`/Game/Blueprints/BP_Playing.AIcnt` _returnvalue_2))
                  (:`  `
                    (set `/Game/Blueprints/BP_Playing.AIcnt` _result_2 _returnvalue_2)
                    (`KismetSystemLibrary.Delay` 2.0)
                    (`self.K2_DestroyActor`)))))))))))

(fn `UserConstructionScript`)