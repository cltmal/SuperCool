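; Stage manager actor that runs a multi-zone VR game through BP_Spawn, spawning player, AI and starting items.
; When Alivecnt matches AIcnt, it has the spawner create the current stage's travel item.
; AllNextPoint advances the ENextStage enum and spawns the next zone, ending with a Missile spawn in Landing.
; Start, zone changes and Restart, which resets to stage one, animate PC_outline's Position and Radius parameters through timelines.
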(event `self.ReceiveTick`
  (params (DeltaSeconds :type "Float (single-precision)"))
  (if (== (`self.Alivecnt`) (`self.AIcnt`))
    (`self.CheckEnemyCount`)
    (set `self.AIcnt` 0)))

(event `self.ReceiveBeginPlay`
  (`WidgetBlueprintLibrary.SetInputMode_GameOnly` (`GameplayStatics.GetPlayerController` 0))
  (bind _returnvalue (`GameplayStatics.GetActorOfClass` "/Game/Blueprints/BP_Spawn.BP_Spawn_C"))
  (set `self.SpwanActor` _returnvalue)
  (`/Game/Blueprints/BP_Spawn.PlayerSpawn1` _returnvalue)
  (`/Game/Blueprints/BP_Spawn.AISpawn1` _returnvalue)
  (`/Game/Blueprints/BP_Spawn.ItemSpawn` _returnvalue)
  (`KismetMaterialLibrary.SetVectorParameterValue` "/Game/Materials/PC_outline.PC_outline" "Position" (`KismetMathLibrary.Conv_VectorToLinearColor` (`SceneComponent.K2_GetComponentLocation` (`self.DefaultSceneRoot`))))
  (`/Engine/EditorBlueprintResources/StandardMacros.FlipFlop`
    (:`A`
      (bind (_direction `_새_트랙_0`) (`Timeline|타임라인_0` :!label _label)
        (:`Update`
          (`KismetMaterialLibrary.SetScalarParameterValue` "/Game/Materials/PC_outline.PC_outline" "Radius" `_새_트랙_0`))))
    (:`B`
      (goto _label :!via `Reverse`))))

(event `CheckEnemyCount`
  (bind _spwanactor (`self.SpwanActor`))
  ;[1 1 1] 다른 지역으로 이동하는 아이템생성
  (switch `/Game/Blueprints/Enum_NextStage` (`self.ENextStage`)
    (:`NewEnumerator0`
      (`/Game/Blueprints/BP_Spawn.GoNextLocation` _spwanactor))
    (:`NewEnumerator2`
      (`/Game/Blueprints/BP_Spawn.GoNextLocation2` _spwanactor))
    (:`NewEnumerator3`
      (`/Game/Blueprints/BP_Spawn.GoNextLocation3` _spwanactor))
    (:`NewEnumerator4`
      (`/Game/Blueprints/BP_Spawn.GoNextLocation4` _spwanactor))
    (:`NewEnumerator6`
      (`/Game/Blueprints/BP_Spawn.GoNextLocation5` _spwanactor))
    (:`NewEnumerator7`
      (`/Game/Blueprints/BP_Spawn.GoNextLocation6` _spwanactor))
    (:`NewEnumerator8`
      (`/Game/Blueprints/BP_Spawn.GoNextLocation7` _spwanactor))))

(event `AllNextPoint`
  ;[1 1 1] 다른 지역으로 이동
  (switch `/Game/Blueprints/Enum_NextStage` (`self.ENextStage`)
    (:`NewEnumerator0`
      (`self.Zone2play`)
      (set `self.ENextStage` "NewEnumerator2")
      (`KismetMaterialLibrary.SetVectorParameterValue` "/Game/Materials/PC_outline.PC_outline" "Position" (`KismetMathLibrary.Conv_VectorToLinearColor` (`SceneComponent.K2_GetComponentLocation` (`/Game/VirtualRealityBP/Blueprints/MotionControllerPawn.Capsule` (cast `/Game/VirtualRealityBP/Blueprints/MotionControllerPawn` (`GameplayStatics.GetPlayerPawn` 0) :!pure true)))) :!label _label_2)
      (bind (_direction `_새_트랙_0`) (`Timeline|타임라인_1` :!via `PlayFromStart`)
        (:`Update`
          (`KismetMaterialLibrary.SetScalarParameterValue` "/Game/Materials/PC_outline.PC_outline" "Radius" `_새_트랙_0`))))
    (:`NewEnumerator2`
      (`self.Zone3play`)
      (set `self.ENextStage` "NewEnumerator3")
      (goto _label_2))
    (:`NewEnumerator3`
      (`self.Zone4play`)
      (set `self.ENextStage` "NewEnumerator4")
      (goto _label_2))
    (:`NewEnumerator4`
      (`self.Zone5Play`)
      (set `self.ENextStage` "NewEnumerator6")
      (goto _label_2))
    (:`NewEnumerator6`
      (`self.Zone6Play`)
      (set `self.ENextStage` "NewEnumerator7")
      (goto _label_2))
    (:`NewEnumerator7`
      (`self.Zone7Play`)
      (set `self.ENextStage` "NewEnumerator8")
      (goto _label_2))
    (:`NewEnumerator8`
      (`self.landing`))))

(event `Restart`
  (set `self.ENextStage` "NewEnumerator0")
  (set `self.AIcnt` 0)
  (`GameplayStatics.SetGamePaused` false)
  (bind _asmotion_controller_pawn (cast `/Game/VirtualRealityBP/Blueprints/MotionControllerPawn` (`GameplayStatics.GetPlayerPawn` 0)))
  (set `/Game/VirtualRealityBP/Blueprints/MotionControllerPawn.isAlive` true _asmotion_controller_pawn)
  (bind _returnvalue (`GameplayStatics.GetActorOfClass` "/Game/Blueprints/BP_Spawn.BP_Spawn_C"))
  (set `self.SpwanActor` _returnvalue)
  (`/Game/Blueprints/BP_Spawn.PlayerSpawn1` _returnvalue)
  (`/Game/Blueprints/BP_Spawn.AISpawn1` _returnvalue)
  (`/Game/Blueprints/BP_Spawn.ItemSpawn` _returnvalue)
  (`KismetMaterialLibrary.SetVectorParameterValue` "/Game/Materials/PC_outline.PC_outline" "Position" (`KismetMathLibrary.Conv_VectorToLinearColor` (`SceneComponent.K2_GetComponentLocation` (`self.DefaultSceneRoot`))))
  (bind (_direction `_새_트랙_0`) (`Timeline|타임라인_2` :!via `PlayFromStart`)
    (:`Update`
      (`KismetMaterialLibrary.SetScalarParameterValue` "/Game/Materials/PC_outline.PC_outline" "Radius" `_새_트랙_0`))))

(fn `landing`
  (bind _returnvalue (`GameplayStatics.GetActorOfClass` "/Game/Blueprints/BP_Spawn.BP_Spawn_C"))
  (`|SpawnActorFromClass` "/Game/launch/missile.missile_C" (`self.GetTransform` (`|GetArrayItem` (`/Game/Blueprints/BP_Spawn.ConeSpawn` _returnvalue) 7)) "AdjustIfPossibleButAlwaysSpawn" "OverrideRootScale" null null))

(fn `UserConstructionScript`)

(fn `Zone2play`
  (bind _returnvalue (`GameplayStatics.GetActorOfClass` "/Game/Blueprints/BP_Spawn.BP_Spawn_C"))
  (`/Game/Blueprints/BP_Spawn.PlayerSpawn2` _returnvalue)
  (`/Game/Blueprints/BP_Spawn.AISpawn2` _returnvalue))

(fn `Zone3play`
  (bind _returnvalue (`GameplayStatics.GetActorOfClass` "/Game/Blueprints/BP_Spawn.BP_Spawn_C"))
  (`/Game/Blueprints/BP_Spawn.PlayerSpawn3` _returnvalue)
  (`/Game/Blueprints/BP_Spawn.AISpawn3` _returnvalue))

(fn `Zone4play`
  (bind _returnvalue (`GameplayStatics.GetActorOfClass` "/Game/Blueprints/BP_Spawn.BP_Spawn_C"))
  (`/Game/Blueprints/BP_Spawn.PlayerSpawn4` _returnvalue)
  (`/Game/Blueprints/BP_Spawn.AISpawn4` _returnvalue))

(fn `Zone5Play`
  (bind _returnvalue (`GameplayStatics.GetActorOfClass` "/Game/Blueprints/BP_Spawn.BP_Spawn_C"))
  (`/Game/Blueprints/BP_Spawn.PlayerSpawn5` _returnvalue)
  (`/Game/Blueprints/BP_Spawn.AISpawn5` _returnvalue))

(fn `Zone6Play`
  (bind _returnvalue (`GameplayStatics.GetActorOfClass` "/Game/Blueprints/BP_Spawn.BP_Spawn_C"))
  (`/Game/Blueprints/BP_Spawn.PlayerSpawn6` _returnvalue)
  (`/Game/Blueprints/BP_Spawn.AISpawn6` _returnvalue))

(fn `Zone7Play`
  (bind _returnvalue (`GameplayStatics.GetActorOfClass` "/Game/Blueprints/BP_Spawn.BP_Spawn_C"))
  (`/Game/Blueprints/BP_Spawn.AISpawn7` _returnvalue)
  (`/Game/Blueprints/BP_Spawn.PlayerSpawn7` _returnvalue))