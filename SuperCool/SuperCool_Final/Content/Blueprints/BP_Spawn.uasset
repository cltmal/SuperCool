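; BP_Spawn is a stage spawner with numbered functions for seven sections, placing enemies, the player and pickups at placed marker actors.
; AISpawn functions spawn pistol and melee AI and set BP_Playing's Alivecnt; later waves reuse references cached by AISpawn1.
; PlayerSpawn teleports the player, GoNextLocation spawns BP_NextItem, and ItemSpawn places laser guns.
; AISpawn5's melee loop has no array connected, and the event graph is empty.
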(event `self.ReceiveBeginPlay`)

(fn `AISpawn1`
  (bind _meleealarray1 (`self.MeleeAlarray1`))
  (bind _aiarray1 (`self.AIarray1`))
  (for _array_element _aiarray1
    (bind _returnvalue (`|SpawnActorFromClass` "/Game/AI/Blueprints/BP_PistolAI.BP_PistolAI_C" (`self.GetTransform` _array_element) "AlwaysSpawn" "OverrideRootScale" null null))
    (set `self.AiPistol` (`GameplayStatics.GetObjectClass` _returnvalue))
    (bind _returnvalue_2 (`GameplayStatics.GetActorOfClass` "/Game/Blueprints/BP_Playing.BP_Playing_C"))
    (set `self.BPplayingActor` _returnvalue_2)
    (set `/Game/Blueprints/BP_Playing.Alivecnt` (+ (`KismetArrayLibrary.Array_Length` _aiarray1) (`KismetArrayLibrary.Array_Length` _meleealarray1)) _returnvalue_2))
  (for _array_element_2 _meleealarray1
    (bind _returnvalue_3 (`|SpawnActorFromClass` "/Game/AI/Blueprints/BP_MeleeAI.BP_MeleeAI_C" (`self.GetTransform` _array_element_2) "Undefined" "OverrideRootScale" null null))
    (set `self.AIMelee` (`GameplayStatics.GetObjectClass` _returnvalue_3))))

(fn `AISpawn2`
  (bind _aiarray2 (`self.AIarray2`))
  (bind _meleealarray2 (`self.MeleeAlarray2`))
  (for _array_element _aiarray2
    (`|SpawnActorFromClass` (`self.AiPistol`) (`self.GetTransform` _array_element) "AdjustIfPossibleButAlwaysSpawn" "OverrideRootScale" null null)
    (set `/Game/Blueprints/BP_Playing.Alivecnt` (+ (`KismetArrayLibrary.Array_Length` _aiarray2) (`KismetArrayLibrary.Array_Length` _meleealarray2)) (`self.BPplayingActor`)))
  (for _array_element_2 _meleealarray2
    (`|SpawnActorFromClass` (`self.AIMelee`) (`self.GetTransform` _array_element_2) "Undefined" "OverrideRootScale" null null)))

(fn `AISpawn3`
  (bind _aiarray3 (`self.AIarray3`))
  (bind _meleealarray3 (`self.MeleeAlarray3`))
  (for _array_element _aiarray3
    (`|SpawnActorFromClass` (`self.AiPistol`) (`self.GetTransform` _array_element) "AdjustIfPossibleButAlwaysSpawn" "OverrideRootScale" null null)
    (set `/Game/Blueprints/BP_Playing.Alivecnt` (+ (`KismetArrayLibrary.Array_Length` _aiarray3) (`KismetArrayLibrary.Array_Length` _meleealarray3)) (`self.BPplayingActor`)))
  (for _array_element_2 _meleealarray3
    (`|SpawnActorFromClass` (`self.AIMelee`) (`self.GetTransform` _array_element_2) "Undefined" "OverrideRootScale" null null)))

(fn `AISpawn4`
  (bind _alarray4 (`self.Alarray4`))
  (bind _meleealarray4 (`self.MeleeAlarray4`))
  (for _array_element _alarray4
    (`|SpawnActorFromClass` (`self.AiPistol`) (`self.GetTransform` _array_element) "AdjustIfPossibleButAlwaysSpawn" "OverrideRootScale" null null)
    (set `/Game/Blueprints/BP_Playing.Alivecnt` (+ (`KismetArrayLibrary.Array_Length` _alarray4) (`KismetArrayLibrary.Array_Length` _meleealarray4)) (`self.BPplayingActor`)))
  (for _array_element_2 _meleealarray4
    (`|SpawnActorFromClass` (`self.AIMelee`) (`self.GetTransform` _array_element_2) "Undefined" "OverrideRootScale" null null)))

(fn `AISpawn5`
  (bind _alarray5 (`self.Alarray5`))
  (for _array_element _alarray5
    (`|SpawnActorFromClass` (`self.AiPistol`) (`self.GetTransform` _array_element) "AlwaysSpawn" "OverrideRootScale" null null)
    (set `/Game/Blueprints/BP_Playing.Alivecnt` (+ (`KismetArrayLibrary.Array_Length` _alarray5) (`KismetArrayLibrary.Array_Length` (`self.MeleeAlarray5`))) (`self.BPplayingActor`)))
  (for _array_element_2 _
    (`|SpawnActorFromClass` (`self.AIMelee`) (`self.GetTransform` _array_element_2) "Undefined" "OverrideRootScale" null null)))

(fn `AISpawn6`
  (bind _meleealarray6 (`self.MeleeAlarray6`))
  (bind _alarray6 (`self.Alarray6`))
  (for _array_element _alarray6
    (`|SpawnActorFromClass` (`self.AiPistol`) (`self.GetTransform` _array_element) "AlwaysSpawn" "OverrideRootScale" null null)
    (set `/Game/Blueprints/BP_Playing.Alivecnt` (+ (`KismetArrayLibrary.Array_Length` _alarray6) (`KismetArrayLibrary.Array_Length` _meleealarray6)) (`self.BPplayingActor`)))
  (for _array_element_2 _meleealarray6
    (`|SpawnActorFromClass` (`self.AIMelee`) (`self.GetTransform` _array_element_2) "Undefined" "OverrideRootScale" null null)))

(fn `AISpawn7`
  (bind _alarray7 (`self.Alarray7`))
  (bind _meleealarray7 (`self.MeleeAlarray7`))
  (for _array_element _alarray7
    (`|SpawnActorFromClass` (`self.AiPistol`) (`self.GetTransform` _array_element) "AlwaysSpawn" "OverrideRootScale" null null)
    (set `/Game/Blueprints/BP_Playing.Alivecnt` (+ (`KismetArrayLibrary.Array_Length` _alarray7) (`KismetArrayLibrary.Array_Length` _meleealarray7)) (`self.BPplayingActor`)))
  (for _array_element_2 _meleealarray7
    (`|SpawnActorFromClass` (`self.AIMelee`) (`self.GetTransform` _array_element_2) "Undefined" "OverrideRootScale" null null)))

(fn `GoNextLocation`
  (for (_array_element _array_index) (`self.ConeSpawn`)
    (if (== _array_index 0)
      (`|SpawnActorFromClass` "/Game/Blueprints/Item/BP_NextItem.BP_NextItem_C" (`self.GetTransform` _array_element) "Undefined" "OverrideRootScale" null null))))

(fn `GoNextLocation2`
  (for (_array_element _array_index) (`self.ConeSpawn`)
    (if (== _array_index 1)
      (`|SpawnActorFromClass` "/Game/Blueprints/Item/BP_NextItem.BP_NextItem_C" (`self.GetTransform` _array_element) "Undefined" "OverrideRootScale" null null))))

(fn `GoNextLocation3`
  (for (_array_element _array_index) (`self.ConeSpawn`)
    (if (== _array_index 2)
      (`|SpawnActorFromClass` "/Game/Blueprints/Item/BP_NextItem.BP_NextItem_C" (`self.GetTransform` _array_element) "Undefined" "OverrideRootScale" null null))))

(fn `GoNextLocation4`
  (for (_array_element _array_index) (`self.ConeSpawn`)
    (if (== _array_index 3)
      (`|SpawnActorFromClass` "/Game/Blueprints/Item/BP_NextItem.BP_NextItem_C" (`self.GetTransform` _array_element) "Undefined" "OverrideRootScale" null null))))

(fn `GoNextLocation5`
  (for (_array_element _array_index) (`self.ConeSpawn`)
    (if (== _array_index 4)
      (`|SpawnActorFromClass` "/Game/Blueprints/Item/BP_NextItem.BP_NextItem_C" (`self.GetTransform` _array_element) "Undefined" "OverrideRootScale" null null))))

(fn `GoNextLocation6`
  (for (_array_element _array_index) (`self.ConeSpawn`)
    (if (== _array_index 5)
      (`|SpawnActorFromClass` "/Game/Blueprints/Item/BP_NextItem.BP_NextItem_C" (`self.GetTransform` _array_element) "Undefined" "OverrideRootScale" null null))))

(fn `GoNextLocation7`
  (`|SpawnActorFromClass` "/Game/Blueprints/Item/BP_NextItem.BP_NextItem_C" (`self.GetTransform` (`|GetArrayItem` (`self.ConeSpawn`) 6)) "AlwaysSpawn" "OverrideRootScale" null null))

(fn `ItemSpawn`
  (for _array_element (`self.ItemArray`)
    (`|SpawnActorFromClass` "/Game/VRGunToolkit/Blueprints/Weapons/Futuristic/BP_LaserGun.BP_LaserGun_C" (`self.GetTransform` _array_element) "Undefined" "OverrideRootScale" null null)))

(fn `PlayerSpawn1`
  (for (_array_element _array_index) (`self.PlayerSpawnPoint`)
    (if (== _array_index 0)
      (`self.K2_TeleportTo` :`self` (`GameplayStatics.GetPlayerPawn` 0) :`DestLocation` (`self.K2_GetActorLocation` _array_element)))))

(fn `PlayerSpawn2`
  (for (_array_element _array_index) (`self.PlayerSpawnPoint`)
    (if (== _array_index 1)
      (`self.K2_TeleportTo` :`self` (`GameplayStatics.GetPlayerPawn` 0) :`DestLocation` (`self.K2_GetActorLocation` _array_element)))))

(fn `PlayerSpawn3`
  (for (_array_element _array_index) (`self.PlayerSpawnPoint`)
    (if (== _array_index 2)
      (`self.K2_TeleportTo` :`self` (`GameplayStatics.GetPlayerPawn` 0) :`DestLocation` (`self.K2_GetActorLocation` _array_element)))))

(fn `PlayerSpawn4`
  (for (_array_element _array_index) (`self.PlayerSpawnPoint`)
    (if (== _array_index 3)
      (`self.K2_TeleportTo` (`GameplayStatics.GetPlayerPawn` 0) (`self.K2_GetActorLocation` _array_element) (struct :`Yaw` 90.0)))))

(fn `PlayerSpawn5`
  (for (_array_element _array_index) (`self.PlayerSpawnPoint`)
    (if (== _array_index 4)
      (`self.K2_TeleportTo` (`GameplayStatics.GetPlayerPawn` 0) (`self.K2_GetActorLocation` _array_element) (struct :`Yaw` -90.0)))))

(fn `PlayerSpawn6`
  (for (_array_element _array_index) (`self.PlayerSpawnPoint`)
    (if (== _array_index 5)
      (`self.K2_TeleportTo` :`self` (`GameplayStatics.GetPlayerPawn` 0) :`DestLocation` (`self.K2_GetActorLocation` _array_element)))))

(fn `PlayerSpawn7`
  (for (_array_element _array_index) (`self.PlayerSpawnPoint`)
    (if (== _array_index 6)
      (`self.K2_TeleportTo` :`self` (`GameplayStatics.GetPlayerPawn` 0) :`DestLocation` (`self.K2_GetActorLocation` _array_element)))))

(fn `UserConstructionScript`)