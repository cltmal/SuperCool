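; BP_NextItem is a touchable sphere item that breaks apart on overlap and calls AllNextPoint on BP_Playing.
; On BeginPlay it creates a canvas render target whose update draws "aTouch!" and feeds it into the sphere's dynamic material.
; On overlap it hides the sphere, adds a destructible mesh and, after a short delay, damages it with a randomized impulse.
; It then disables sphere collision, notifies BP_Playing and immediately destroys itself.
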(event `self.ReceiveBeginPlay`
  (bind _returnvalue (`CanvasRenderTarget2D.CreateCanvasRenderTarget2D` "/Script/Engine.CanvasRenderTarget2D"))
  (bind _output_get (set `self.Text` _returnvalue))
  (add `CanvasRenderTarget2D.OnCanvasRenderTargetUpdate` _output_get (delegate `DrawTextAtTexture`))
  (`CanvasRenderTarget2D.UpdateResource` _returnvalue))

(event `DrawTextAtTexture`
  (params (Canvas :type "Canvas Object Reference") (Width :type Integer) (Height :type Integer))
  (bind _sphere (`self.Sphere`))
  (`Canvas.K2_DrawText` Canvas "/Engine/EngineFonts/Roboto.Roboto" "aTouch!" (-50.0 300.0) (7.0 7.0) (struct :`R` 1.0 :`B` 0.288342 :`A` 1.0) 0.0 (struct :`A` 1.0) (1.0 1.0) false false false (struct :`A` 1.0))
  (bind _returnvalue (`PrimitiveComponent.CreateDynamicMaterialInstance` _sphere 0 (`PrimitiveComponent.GetMaterial` _sphere 0) "None"))
  (`PrimitiveComponent.SetMaterial` _sphere 0 _returnvalue)
  (`MaterialInstanceDynamic.SetTextureParameterValue` _returnvalue "PT2D" (`self.Text`)))

(event `self.Sphere.OnComponentBeginOverlap`
  (params (OverlappedComponent :type "PrimitiveComponent Object Reference") (OtherActor :type "Actor Object Reference") (OtherComp :type "PrimitiveComponent Object Reference") (OtherBodyIndex :type Integer) (bFromSweep :type Boolean) (SweepResult :type "HitResult Structure (by ref)"))
  (`SceneComponent.SetVisibility` (`self.Sphere`) false false)
  (bind _returnvalue (`AddComponent|NODE_AddDestructibleComponent-0` :`RelativeTransform` (`SceneComponent.GetRelativeTransform` (`self.Sphere`))))
  (`DestructibleComponent.SetDestructibleMesh` _returnvalue "/Engine/BasicShapes/Sphere_DM.Sphere_DM")
  (`KismetSystemLibrary.Delay` 0.1)
  (`PrimitiveComponent.SetSimulatePhysics` _returnvalue true)
  (`DestructibleComponent.ApplyDamage` _returnvalue 60.0 (`SceneComponent.K2_GetComponentLocation` (`self.Sphere`)) (`KismetMathLibrary.MakeVector` (`KismetMathLibrary.SelectFloat` 0.0 1.0 (`KismetMathLibrary.RandomBool`)) (`KismetMathLibrary.SelectFloat` 0.0 1.0 (`KismetMathLibrary.RandomBool`)) (`KismetMathLibrary.SelectFloat` 0.0 1.0 (`KismetMathLibrary.RandomBool`))) 600.0)
  (`PrimitiveComponent.SetCollisionEnabled` (`self.Sphere`) "NoCollision")
  (bind _returnvalue_2 (`GameplayStatics.GetActorOfClass` "/Game/Blueprints/BP_Playing.BP_Playing_C"))
  (`/Game/Blueprints/BP_Playing.AllNextPoint` _returnvalue_2)
  (`self.K2_DestroyActor`))

(fn `UserConstructionScript`)