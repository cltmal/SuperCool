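; Two-floor elevator Blueprint with sliding cabin and landing doors and button materials that show call and travel state.
; Timelines move the doors and raise or lower the cabin by FloorHeight, with Delays on their Update pins sequencing arrival, opening and timed closing.
; BeginPlay opens the downstairs doors.
; Button and cabin overlap events and downstairs closing are empty; their logic, including call/launch dispatch, sits in unconnected nodes that never run.
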(event `Open_Door_US`
  (bind _door_wait_time (`self.Door_Wait_Time`))
  ;[1 1 1] Open Door Upstair
  (set `self.Active` true)
  (if (not (`self.DoorOpened`))
    (`PrimitiveComponent.SetMaterial` (`self.Upstair_Elevator_Case`) 2 "/Game/Corridor/Materials/MAT_Call_Button_US_Launch.MAT_Call_Button_US_Launch")
    (`PrimitiveComponent.SetMaterial` (`self.SM_Elevator_Case`) 2 "/Game/Corridor/Materials/MAT_Call_Button_US_Launch.MAT_Call_Button_US_Launch")
    (bind (_direction _0_to_70) (`Timeline|Timeline_4` :!via `PlayFromStart`)
      (:`Update`
        (bind _returnvalue (- (`self.Left_Doors_SP`) _0_to_70))
        (`SceneComponent.K2_SetRelativeTransform` (`self.SM_Indoor_L`) (`KismetMathLibrary.MakeTransform` (`KismetMathLibrary.MakeVector` _returnvalue)) false false)
        (`SceneComponent.K2_SetRelativeTransform` (`self.Upstair_L`) (`KismetMathLibrary.MakeTransform` (`KismetMathLibrary.MakeVector` _returnvalue)) false false)
        (set `self.Left_Doors_NP` _returnvalue)
        (bind _returnvalue_2 (+ (`self.Right_Doors_SP`) _0_to_70))
        (`SceneComponent.K2_SetRelativeTransform` (`self.SM_Indoor_R`) (`KismetMathLibrary.MakeTransform` (`KismetMathLibrary.MakeVector` _returnvalue_2)) false false)
        (`SceneComponent.K2_SetRelativeTransform` (`self.Upstair_R`) (`KismetMathLibrary.MakeTransform` (`KismetMathLibrary.MakeVector` _returnvalue_2)) false false)
        (set `self.Right_Doors_NP` _returnvalue_2)
        (`KismetSystemLibrary.Delay` 3.0)
        (set `self.DoorOpened` true)
        (`KismetSystemLibrary.Delay` _door_wait_time)
        (set `self.Active` false)
        (if (`self.InElevator?`) :!label _label
          (if (`self.DoorOpened`)
            (`KismetSystemLibrary.Delay` _door_wait_time)
            (goto _label))
          (else
            (`self.Close_Door_US`)))))))

(event `Open_Door_DS`
  (bind _door_wait_time (`self.Door_Wait_Time`))
  ;[1 1 1] Open Door Downstair
  (set `self.Active` true)
  (if (not (`self.DoorOpened`))
    (`PrimitiveComponent.SetMaterial` (`self.Upstair_Elevator_Case`) 2 "/Game/Corridor/Materials/MAT_Call_Button_DS_Launch.MAT_Call_Button_DS_Launch")
    (`PrimitiveComponent.SetMaterial` (`self.SM_Elevator_Case`) 2 "/Game/Corridor/Materials/MAT_Call_Button_DS_Launch.MAT_Call_Button_DS_Launch")
    (bind (_direction _0_to_70) (`Timeline|Timeline_2` :!via `PlayFromStart`)
      (:`Update`
        (bind _returnvalue (- (`self.Left_Doors_SP`) _0_to_70))
        (`SceneComponent.K2_SetRelativeTransform` (`self.SM_Outdoor_L`) (`KismetMathLibrary.MakeTransform` (`KismetMathLibrary.MakeVector` _returnvalue)) true false)
        (`SceneComponent.K2_SetRelativeTransform` (`self.SM_Indoor_L`) (`KismetMathLibrary.MakeTransform` (`KismetMathLibrary.MakeVector` _returnvalue)) true false)
        (set `self.Left_Doors_NP` _returnvalue)
        (bind _returnvalue_2 (+ (`self.Right_Doors_SP`) _0_to_70))
        (`SceneComponent.K2_SetRelativeTransform` (`self.SM_Indoor_R`) (`KismetMathLibrary.MakeTransform` (`KismetMathLibrary.MakeVector` _returnvalue_2)) true false)
        (`SceneComponent.K2_SetRelativeTransform` (`self.SM_Outdoor_R`) (`KismetMathLibrary.MakeTransform` (`KismetMathLibrary.MakeVector` _returnvalue_2)) true false)
        (set `self.Right_Doors_NP` _returnvalue_2)
        (`KismetSystemLibrary.Delay` 3.0)
        (set `self.DoorOpened` true)
        (`KismetSystemLibrary.Delay` _door_wait_time)
        (set `self.Active` false)
        (if (`self.InElevator?`) :!label _label_2
          (if (`self.DoorOpened`)
            (`KismetSystemLibrary.Delay` _door_wait_time)
            (goto _label_2))
          (else
            (`self.Close_Door_DS`)))))))

(event `self.ReceiveBeginPlay`
  (bind (_returnvalue_x _returnvalue_y _returnvalue_z) (`KismetMathLibrary.BreakVector` (`self.K2_GetActorLocation`)))
  (set `self.Start_Location_Z` _returnvalue_z)
  (set `self.Right_Doors_SP` (.x (.location (`SceneComponent.GetRelativeTransform` (`self.SM_Indoor_R`)))))
  (set `self.Left_Doors_SP` (.x (.location (`SceneComponent.GetRelativeTransform` (`self.SM_Indoor_L`)))))
  (`KismetSystemLibrary.Delay` 3.0)
  (`self.Open_Door_DS`))

(event `Close_Door_DS`
  ;[1 1 1] Close Door Downstair
)

(event `Close_Door_US`
  ;[1 1 1] Close Door Upstair
  (if (`self.DoorOpened`)
    (set `self.Active` true)
    (bind (_direction _0_to_70) (`Timeline|Timeline_5` :!via `PlayFromStart`)
      (:`Update`
        (`SceneComponent.K2_SetRelativeTransform` (`self.SM_Indoor_L`) (`KismetMathLibrary.MakeTransform` (`KismetMathLibrary.MakeVector` (+ (`self.Left_Doors_NP`) _0_to_70))) false false)
        (`SceneComponent.K2_SetRelativeTransform` (`self.Upstair_L`) (`KismetMathLibrary.MakeTransform` (`KismetMathLibrary.MakeVector` (+ (`self.Left_Doors_NP`) _0_to_70))) false false)
        (`SceneComponent.K2_SetRelativeTransform` (`self.SM_Indoor_R`) (`KismetMathLibrary.MakeTransform` (`KismetMathLibrary.MakeVector` (- (`self.Right_Doors_NP`) _0_to_70))) false false)
        (`SceneComponent.K2_SetRelativeTransform` (`self.Upstair_R`) (`KismetMathLibrary.MakeTransform` (`KismetMathLibrary.MakeVector` (- (`self.Right_Doors_NP`) _0_to_70))) false false)
        (`KismetSystemLibrary.Delay` 3.0)
        (set `self.DoorOpened` false)
        (`PrimitiveComponent.SetMaterial` (`self.Upstair_Elevator_Case`) 2 "/Game/Corridor/Materials/MAT_Call_Button_US.MAT_Call_Button_US")
        (`PrimitiveComponent.SetMaterial` (`self.SM_Elevator_Case`) 2 "/Game/Corridor/Materials/MAT_Call_Button_US.MAT_Call_Button_US")
        (set `self.Active` false)))))

(event `self.Button.OnComponentBeginOverlap`
  (params (OverlappedComponent :type "PrimitiveComponent Object Reference") (OtherActor :type "Actor Object Reference") (OtherComp :type "PrimitiveComponent Object Reference") (OtherBodyIndex :type Integer) (bFromSweep :type Boolean) (SweepResult :type "HitResult Structure (by ref)")))

(event `self.Button.OnComponentEndOverlap`
  (params (OverlappedComponent :type "PrimitiveComponent Object Reference") (OtherActor :type "Actor Object Reference") (OtherComp :type "PrimitiveComponent Object Reference") (OtherBodyIndex :type Integer)))

(event `Key|E`
  (params (Key :type "Key Structure"))
  ;[1 1 1] Launch Key
)

(event `Launch4Down`
  ;[1 1 1] Launch Elevator
  (set `self.Active` true)
  (`PrimitiveComponent.SetMaterial` (`self.Upstair_Elevator_Case`) 2 "/Game/Corridor/Materials/MAT_Call_Button_DS_Launch.MAT_Call_Button_DS_Launch")
  (`PrimitiveComponent.SetMaterial` (`self.SM_Elevator_Case`) 2 "/Game/Corridor/Materials/MAT_Call_Button_DS_Launch.MAT_Call_Button_DS_Launch")
  (`PrimitiveComponent.SetMaterial` (`self.SM_Elevator`) 3 "/Game/Corridor/Materials/MAT_Buttons_GoDS.MAT_Buttons_GoDS")
  (`KismetSystemLibrary.Delay` 3.1)
  (bind (_direction _newtrack_0) (`Timeline|Timeline_1` :!via `ReverseFromEnd`)
    (:`Update`
      (`SceneComponent.K2_SetRelativeTransform` (`self.SM_Elevator`) (`KismetMathLibrary.MakeTransform` (`KismetMathLibrary.MakeVector` 180.0 -27.0 (* _newtrack_0 (`self.Floor_Height`)))) false false)
      (`KismetSystemLibrary.Delay` 5.5)
      (set `self.Upstair` false)
      (`PrimitiveComponent.SetMaterial` (`self.SM_Elevator`) 3 "/Game/Corridor/Materials/MAT_Buttons_OnDS.MAT_Buttons_OnDS")
      (`self.Open_Door_DS`))))

(event `self.CallButton.OnComponentBeginOverlap`
  (params (OverlappedComponent :type "PrimitiveComponent Object Reference") (OtherActor :type "Actor Object Reference") (OtherComp :type "PrimitiveComponent Object Reference") (OtherBodyIndex :type Integer) (bFromSweep :type Boolean) (SweepResult :type "HitResult Structure (by ref)")))

(event `self.CallButton.OnComponentEndOverlap`
  (params (OverlappedComponent :type "PrimitiveComponent Object Reference") (OtherActor :type "Actor Object Reference") (OtherComp :type "PrimitiveComponent Object Reference") (OtherBodyIndex :type Integer)))

(event `self.InElevator.OnComponentBeginOverlap`
  (params (OverlappedComponent :type "PrimitiveComponent Object Reference") (OtherActor :type "Actor Object Reference") (OtherComp :type "PrimitiveComponent Object Reference") (OtherBodyIndex :type Integer) (bFromSweep :type Boolean) (SweepResult :type "HitResult Structure (by ref)")))

(event `self.InElevator.OnComponentEndOverlap`
  (params (OverlappedComponent :type "PrimitiveComponent Object Reference") (OtherActor :type "Actor Object Reference") (OtherComp :type "PrimitiveComponent Object Reference") (OtherBodyIndex :type Integer)))

(event `self.Upstair_CallButton.OnComponentBeginOverlap`
  (params (OverlappedComponent :type "PrimitiveComponent Object Reference") (OtherActor :type "Actor Object Reference") (OtherComp :type "PrimitiveComponent Object Reference") (OtherBodyIndex :type Integer) (bFromSweep :type Boolean) (SweepResult :type "HitResult Structure (by ref)")))

(event `Launch4Up`
  ;[1 1 1] Launch Elevator
  (set `self.Active` true)
  (`PrimitiveComponent.SetMaterial` (`self.Upstair_Elevator_Case`) 2 "/Game/Corridor/Materials/MAT_Call_Button_US_Launch.MAT_Call_Button_US_Launch")
  (`PrimitiveComponent.SetMaterial` (`self.SM_Elevator_Case`) 2 "/Game/Corridor/Materials/MAT_Call_Button_US_Launch.MAT_Call_Button_US_Launch")
  (`PrimitiveComponent.SetMaterial` (`self.SM_Elevator`) 3 "/Game/Corridor/Materials/MAT_Buttons_GoUS.MAT_Buttons_GoUS")
  (`KismetSystemLibrary.Delay` 3.1)
  (bind (_direction _newtrack_0) (`Timeline|Timeline_0` :!via `PlayFromStart`)
    (:`Update`
      (`SceneComponent.K2_SetRelativeTransform` (`self.SM_Elevator`) (`KismetMathLibrary.MakeTransform` (`KismetMathLibrary.MakeVector` 180.0 -27.0 (* _newtrack_0 (`self.Floor_Height`)))) false false)
      (`KismetSystemLibrary.Delay` 5.5)
      (set `self.Upstair` true)
      (`PrimitiveComponent.SetMaterial` (`self.SM_Elevator`) 3 "/Game/Corridor/Materials/MAT_Buttons_OnUS.MAT_Buttons_OnUS")
      (`self.Open_Door_US`))))

(event `self.Upstair_CallButton.OnComponentEndOverlap`
  (params (OverlappedComponent :type "PrimitiveComponent Object Reference") (OtherActor :type "Actor Object Reference") (OtherComp :type "PrimitiveComponent Object Reference") (OtherBodyIndex :type Integer)))

(fn `UserConstructionScript`)