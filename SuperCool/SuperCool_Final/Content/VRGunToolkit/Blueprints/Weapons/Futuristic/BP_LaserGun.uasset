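; Laser gun weapon Blueprint for player and AI use, extending a parent gun class with a muzzle-flash-style material glow.
; Construction creates a dynamic material on Frame; each fire event briefly spikes its EmissiveIntensity around the parent's firing call.
; MoveToPlayer computes an arced launch velocity toward the player and debug-draws the predicted path, without moving the gun.
; ChangeMatetialforItem reapplies the static material; spline and interpolated-movement logic is left unconnected.
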(event `MoveToPlayer`
  (bind _outlaunchvelocity (`GameplayStatics.SuggestProjectileVelocity_CustomArc` (`SceneComponent.K2_GetComponentLocation` (`self.Frame`)) (`self.K2_GetActorLocation` (`GameplayStatics.GetPlayerPawn` 0)) 0.0 0.7))
  (set `self.Destination` _outlaunchvelocity)
  (`GameplayStatics.Blueprint_PredictProjectilePath_ByTraceChannel` :`StartPos` (`SceneComponent.K2_GetComponentLocation` (`self.Frame`)) :`LaunchVelocity` (`self.Destination`) :`bTracePath` false :`ProjectileRadius` 20.0 :`DrawDebugType` "ForDuration"))

(event `self.ReceiveBeginPlay`)

(event `self.Fire`
  (bind _dynamicguntexture (`self.DynamicGunTexture`))
  ;[0.5571 1 0.696] Material Animation Example, the gun glows everytime we shoot
  (`MaterialInstanceDynamic.SetScalarParameterValue` _dynamicguntexture "EmissiveIntensity" 5.0)
  (`parent.Fire`)
  (`KismetSystemLibrary.Delay` 0.05)
  (`MaterialInstanceDynamic.SetScalarParameterValue` _dynamicguntexture "EmissiveIntensity" 1.0))

(event `self.FireLoop`
  (bind _dynamicguntexture (`self.DynamicGunTexture`))
  ;[0.5571 1 0.696] Material Animation Example, the gun glows everytime we shoot
  (`parent.FireLoop`)
  (`MaterialInstanceDynamic.SetScalarParameterValue` _dynamicguntexture "EmissiveIntensity" 5.0)
  (`KismetSystemLibrary.Delay` 0.05)
  (`MaterialInstanceDynamic.SetScalarParameterValue` _dynamicguntexture "EmissiveIntensity" 1.0))

(event `self.AiFire`
  (bind _dynamicguntexture (`self.DynamicGunTexture`))
  (`MaterialInstanceDynamic.SetScalarParameterValue` _dynamicguntexture "EmissiveIntensity" 5.0)
  (`parent.AiFire`)
  (`KismetSystemLibrary.Delay` 0.05)
  (`MaterialInstanceDynamic.SetScalarParameterValue` _dynamicguntexture "EmissiveIntensity" 1.0))

(event `/Game/Weapon/InteractableInterface.ActionLeftWeapon`
  (bind _dynamicguntexture (`self.DynamicGunTexture`))
  (`MaterialInstanceDynamic.SetScalarParameterValue` _dynamicguntexture "EmissiveIntensity" 5.0)
  (`parent.PlayerLeftShot`)
  (`KismetSystemLibrary.Delay` 0.05)
  (`MaterialInstanceDynamic.SetScalarParameterValue` _dynamicguntexture "EmissiveIntensity" 1.0))

(event `/Game/Weapon/InteractableInterface.ActionRightWeapon`
  (bind _dynamicguntexture (`self.DynamicGunTexture`))
  (`MaterialInstanceDynamic.SetScalarParameterValue` _dynamicguntexture "EmissiveIntensity" 5.0)
  (`parent.PlayerRightShot`)
  (`KismetSystemLibrary.Delay` 0.05)
  (`MaterialInstanceDynamic.SetScalarParameterValue` _dynamicguntexture "EmissiveIntensity" 1.0))

(event `/Game/VirtualRealityBP/Blueprints/ItemMaterial.changeMatetial for item`
  (`PrimitiveComponent.SetMaterial` (`self.Frame`) 0 "/Game/VRGunToolkit/Materials/Weapons/Futuristic/M_Light_ambient_occlusion_Mat.M_Light_ambient_occlusion_Mat"))

(fn `UserConstructionScript`
  (`parent.UserConstructionScript`)
  (bind _returnvalue (`PrimitiveComponent.CreateDynamicMaterialInstance` (`self.Frame`) 0 "/Game/VRGunToolkit/Materials/Weapons/Futuristic/M_Light_ambient_occlusion_Mat.M_Light_ambient_occlusion_Mat" "None"))
  (set `self.DynamicGunTexture` _returnvalue))