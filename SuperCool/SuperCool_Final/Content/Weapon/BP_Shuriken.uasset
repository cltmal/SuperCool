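; VR shuriken weapon that attaches to either motion controller hand and can be dropped as a throwable.
; Drop re-enables physics and derives force vectors from hand velocities, both using the left hand's direction, but applies a zero impulse.
; Actor hits after a drop deal damage.
; Component hits with a large enough stored force swap the mesh for a fracturing Uzi destructible, then destroy the actor after a delay.
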(event `/Game/VirtualRealityBP/Blueprints/PickupActorInterface.PickupRightHand`
  (params (AttachToRight :type "SceneComponent Object Reference"))
  (`PrimitiveComponent.SetSimulatePhysics` (`self.StaticMeshComponent`) false)
  (`SceneComponent.K2_AttachToComponent` (`self.K2_GetRootComponent`) AttachToRight "None" "SnapToTarget" "SnapToTarget" "KeepWorld" false)
  (`SceneComponent.K2_SetRelativeLocationAndRotation` :`self` (`self.StaticMeshComponent`) :`NewLocation` (-4.0 0.0 -3.0))
  (set `/Game/VirtualRealityBP/Blueprints/MotionControllerPawn.Item Right Hand` self (cast `/Game/VirtualRealityBP/Blueprints/MotionControllerPawn` (`GameplayStatics.GetPlayerPawn` 0) :!pure true)))

(event `/Game/VirtualRealityBP/Blueprints/PickupActorInterface.PickupLeftHand`
  (params (AttachToLeft :type "SceneComponent Object Reference"))
  (`PrimitiveComponent.SetSimulatePhysics` (`self.StaticMeshComponent`) false)
  (`SceneComponent.K2_AttachToComponent` (`self.K2_GetRootComponent`) AttachToLeft "None" "SnapToTarget" "SnapToTarget" "KeepWorld" false)
  (`SceneComponent.K2_SetRelativeLocationAndRotation` :`self` (`self.StaticMeshComponent`) :`NewLocation` (-4.0 0.0 -3.0))
  (set `/Game/VirtualRealityBP/Blueprints/MotionControllerPawn.ItemLeft Hand` self (cast `/Game/VirtualRealityBP/Blueprints/MotionControllerPawn` (`GameplayStatics.GetPlayerPawn` 0) :!pure true)))

(event `/Game/VirtualRealityBP/Blueprints/PickupActorInterface.Drop`
  ;[1 1 1] 아이템을 던지고 맞았을때 Hit이벤트 불러오기
  (add `self.OnActorHit` (delegate `ThrowWeaponHit`))
  (`PrimitiveComponent.SetSimulatePhysics` (`self.StaticMeshComponent`) true)
  (`self.K2_DetachFromActor` "KeepWorld" "KeepWorld" "KeepWorld")
  (bind _returnvalue (`GameplayStatics.GetActorOfClass` "/Game/VirtualRealityBP/Blueprints/BP_MotionController.BP_MotionController_C"))
  (bind _returnvalue_2 (`GameplayStatics.GetActorOfClass` "/Game/VirtualRealityBP/Blueprints/MotionControllerPawn.MotionControllerPawn_C"))
  (bind _returnvalue_3 (`SceneComponent.GetForwardVector` (`/Game/VirtualRealityBP/Blueprints/BP_MotionController.HandMesh` (`/Game/VirtualRealityBP/Blueprints/MotionControllerPawn.LeftController` _returnvalue_2))))
  (set `self.Left ForceVector` (* _returnvalue_3 (* (`KismetMathLibrary.VSize` (`/Game/VirtualRealityBP/Blueprints/BP_MotionController.LeftHandVelocity` _returnvalue)) 5.0)))
  (set `self.Right ForceVector` (* _returnvalue_3 (* (`KismetMathLibrary.VSize` (`/Game/VirtualRealityBP/Blueprints/BP_MotionController.RightHandVelocity` _returnvalue)) 5.0)))
  (`PrimitiveComponent.AddImpulseAtLocation` (`self.StaticMeshComponent`) (0.0 0.0 0.0) (0.0 0.0 0.0) "None"))

(event `ThrowWeaponHit` :!signature `self.OnActorHit`
  (params (SelfActor :type "Actor Object Reference") (OtherActor :type "Actor Object Reference") (NormalImpulse :type "Vector Structure") (Hit :type "HitResult Structure (by ref)"))
  ;[1 1 1] 아이템을 던지고 맞았을때 Hit이벤트 불러오기
  (`GameplayStatics.ApplyDamage` OtherActor 1.0 (`GameplayStatics.GetPlayerController` 0) (`GameplayStatics.GetPlayerPawn` 0)))

(event `/Game/VirtualRealityBP/Blueprints/ItemMaterial.changeMatetial for item`
  ;[1 1 1] 손에 있는게 BP_Uzi3 이면  Uzi3의 색상을 바꾼다
  (bind _returnvalue (`GameplayStatics.GetActorOfClass` "/Game/VirtualRealityBP/Blueprints/MotionControllerPawn.MotionControllerPawn_C"))
  (if (`KismetStringLibrary.EqualEqual_StrStr` (`KismetSystemLibrary.GetDisplayName` (`/Game/VirtualRealityBP/Blueprints/MotionControllerPawn.Item Right Hand` _returnvalue)) "BP_Shuriken")
    (`PrimitiveComponent.SetMaterial` (`self.StaticMeshComponent`) 0 "/Game/FPS_Weapon_Bundle/Weapons/Materials/SMG11/M_SMG11.M_SMG11")))

(event `self.StaticMeshComponent.OnComponentHit`
  (params (HitComponent :type "PrimitiveComponent Object Reference") (OtherActor :type "Actor Object Reference") (OtherComp :type "PrimitiveComponent Object Reference") (NormalImpulse :type "Vector Structure") (Hit :type "HitResult Structure (by ref)"))
  (bind _left_forcevector (`self.Left ForceVector`))
  (bind _right_forcevector (`self.Right ForceVector`))
  ;[1 1 1] 총이 어딘가에 히트 됬을때 일정조건이상의 속도가 나오지않으면 부셔지지않는다
  (`|ExecutionSequence`
    (:`then_0`
      (if (`KismetMathLibrary.Vector_IsNearlyZero` _left_forcevector 0.05)
        _
        (elif (>= (`KismetMathLibrary.VSize` _left_forcevector) 9.0)
          (`/Engine/EditorBlueprintResources/StandardMacros.DoOnce` false
            (:`Completed`
              (`self.WeaponDestructibles `)
              (`KismetSystemLibrary.Delay` 1.5)
              (`self.K2_DestroyActor`))))))
    (:`then_1`
      (if (`KismetMathLibrary.Vector_IsNearlyZero` _right_forcevector 0.05)
        _
        (elif (>= (`KismetMathLibrary.VSize` _right_forcevector) 9.0)
          (`/Engine/EditorBlueprintResources/StandardMacros.DoOnce` false
            (:`Completed`
              (`self.WeaponDestructibles `)
              (`KismetSystemLibrary.Delay` 1.5)
              (`self.K2_DestroyActor`))))))))

(fn `UserConstructionScript`)

(fn `WeaponDestructibles `
  (locals (NewLocalVar_0 :type "DestructibleMesh Object Reference" :default "DestructibleMesh'/Game/Weapon/Uzi_Mesh_DM.Uzi_Mesh_DM'"))
  (`SceneComponent.SetVisibility` (`self.StaticMeshComponent`) false false)
  (bind _returnvalue (`AddComponent|NODE_AddDestructibleComponent-3` :`bManualAttachment` true :`RelativeTransform` (`SceneComponent.GetRelativeTransform` (`self.StaticMeshComponent`))))
  (`DestructibleComponent.SetDestructibleMesh` _returnvalue "/Game/Weapon/Uzi_Mesh_DM.Uzi_Mesh_DM")
  (`PrimitiveComponent.SetSimulatePhysics` _returnvalue true)
  (`DestructibleComponent.ApplyDamage` _returnvalue 10.0 (`SceneComponent.K2_GetComponentLocation` (`self.StaticMeshComponent`)) (`KismetMathLibrary.MakeVector` (`KismetMathLibrary.SelectFloat` 0.0 1.0 (`KismetMathLibrary.RandomBool`)) (`KismetMathLibrary.SelectFloat` 0.0 1.0 (`KismetMathLibrary.RandomBool`)) (`KismetMathLibrary.SelectFloat` 0.0 1.0 (`KismetMathLibrary.RandomBool`))) 100.0)
  (`PrimitiveComponent.SetCollisionEnabled` (`self.StaticMeshComponent`) "NoCollision"))